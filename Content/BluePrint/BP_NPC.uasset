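; Quest NPC that shows dialog and magic options to the VR pawn, driven by its DataIndex entry in BP_NPCManager.
; On BeginPlay, if bQuestClesr is set, its magic type selects a hard-coded layout of movement, loop and numbered block spawners, plus BP_Ice for type 1.
; Trigger overlap feeds the entry into the dialog, quest option and magic option widgets.
; Leaving the trigger hides all three widgets.
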(event OnComponentEndOverlap(Triger)
  (params (OverlappedComponent :type Primitive%20Component%20Object%20Reference) (OtherActor :type Actor%20Object%20Reference) (OtherComp :type Primitive%20Component%20Object%20Reference) (OtherBodyIndex :type Integer))
  (Widget|SetVisibility (Variables|Default|GetAs%20WBP%20NPCDialog) "Hidden")
  (Widget|SetVisibility (Variables|Default|GetAs%20WBP%20Dialog%20Option) "Hidden")
  (Widget|SetVisibility (Variables|Default|GetAs%20WBP%20Magic%20Option) "Hidden")
  (Variables|Default|SetOverLap false))

(event OnComponentBeginOverlap(Triger)
  (params (OverlappedComponent :type Primitive%20Component%20Object%20Reference) (OtherActor :type Actor%20Object%20Reference) (OtherComp :type Primitive%20Component%20Object%20Reference) (OtherBodyIndex :type Integer) (bFromSweep :type Boolean) (SweepResult :type Hit%20Result%20Structure%20%28by%20ref%29))
  (bind _datamgr (Variables|Default|GetDataMgr))
  (bind _dataindex (Variables|Default|GetDataIndex))
  (bind _npcdata (Variables|/Game/BluePrint/NPC/BP_NPCManager.BP_NPCManager_C|GetNPCData _datamgr))
  (bind _output (Utilities|Array|Get(acopy) _npcdata _dataindex))
  (Utilities|Casting|CastToVRPawn OtherActor)
  (bind _output_get (Variables|Default|SetOverLap true))
  (Widget|SetVisibility (Variables|Default|GetAs%20WBP%20NPCDialog) "Visible")
  (Default|UpdateDialog (Variables|Default|GetAs%20WBP%20NPCDialog) (.nickname _output) (.name _output) (.dialog _output) (.firstdialog _output) (.bquestclesr _output))
  (Default|QuestOptionVisiblity (Variables|Default|GetAs%20WBP%20Dialog%20Option) (and (.bquestclesr _output) _output_get))
  (Default|SetMagicType (Variables|Default|GetAs%20WBP%20Magic%20Option) (.mgictype _output) _dataindex (.magicclicletransform _output) (.algorithmtransform _output) (.magicwidgettransform _output)))

(event EventBeginPlay
  (|CallParentFunction)
  (bind _returnvalue (Actor|GetActorOfClass "/Game/BluePrint/NPC/BP_NPCManager.BP_NPCManager_C"))
  (Variables|Default|SetDataMgr _returnvalue)
  (if (.bquestclesr (Utilities|Array|Get(acopy) (Variables|/Game/BluePrint/NPC/BP_NPCManager.BP_NPCManager_C|GetNPCData (Variables|Default|GetDataMgr)) (Variables|Default|GetDataIndex)))
    (switch int (.mgictype (Utilities|Array|Get(acopy) (Variables|/Game/BluePrint/NPC/BP_NPCManager.BP_NPCManager_C|GetNPCData (Variables|Default|GetDataMgr)) (Variables|Default|GetDataIndex)))
      (:0
        (CallFunction|SpawnBlockSpawner1))
      (:1
        (Game|SpawnActorfromClass "/Game/BluePrint/NPC/BP_Ice.BP_Ice_C" (Math|Transform|MakeTransform "-6980.000000,2510.000000,80.000000" "0, 0, 0" "1.000000,1.000000,1.000000") "Undefined" "MultiplyWithRoot" 0 0)
        (CallFunction|SpawnBlockSpawner2)))))

(fn ConstructionScript
  (|CallParentFunction))

(fn SpawnBlockSpawner2
  (Utilities|FlowControl|Sequence
    (:then_0
      (Game|SpawnActorfromClass "/Game/BluePrint/spawner/BP_spawner_Forword.BP_spawner_Forword_C" (Math|Transform|MakeTransform "-6520.000000,2750.000000,180.000000" "0, 0, 0" "0.100000,0.100000,0.100000") "Undefined" "MultiplyWithRoot" 0 0)
      (Game|SpawnActorfromClass "/Game/BluePrint/spawner/BP_spawner_Jump.BP_spawner_Jump_C" (Math|Transform|MakeTransform "-6570.000000,2750.000000,180.000000" "0, 0, 0" "0.100000,0.100000,0.100000") "Undefined" "MultiplyWithRoot" 0 0)
      (Game|SpawnActorfromClass "/Game/BluePrint/spawner/BP_spawner_LeftTurn.BP_spawner_LeftTurn_C" (Math|Transform|MakeTransform "-6620.000000,2750.000000,180.000000" "0, 0, 0" "0.100000,0.100000,0.100000") "Undefined" "MultiplyWithRoot" 0 0)
      (Game|SpawnActorfromClass "/Game/BluePrint/spawner/BP_spawner_RightTurn.BP_spawner_RightTurn_C" (Math|Transform|MakeTransform "-6670.000000,2750.000000,180.000000" "0, 0, 0" "0.100000,0.100000,0.100000") "Undefined" "MultiplyWithRoot" 0 0))
    (:then_1
      (Game|SpawnActorfromClass "/Game/BluePrint/spawner/BP_spawner_Loop.BP_spawner_Loop_C" (Math|Transform|MakeTransform "-6520.000000,2750.000000,140.000000" "0, 0, 0" "0.100000,0.100000,0.100000") "Undefined" "MultiplyWithRoot" 0 0)
      (Game|SpawnActorfromClass "/Game/BluePrint/spawner/BP_spawner_2.BP_spawner_2_C" (Math|Transform|MakeTransform "-6570.000000,2750.000000,140.000000" "0, 0, 0" "0.100000,0.100000,0.100000") "Undefined" "MultiplyWithRoot" 0 0)
      (Game|SpawnActorfromClass "/Game/BluePrint/spawner/BP_spawner_3.BP_spawner_3_C" (Math|Transform|MakeTransform "-6620.000000,2750.000000,140.000000" "0, 0, 0" "0.100000,0.100000,0.100000") "Undefined" "MultiplyWithRoot" 0 0)
      (Game|SpawnActorfromClass "/Game/BluePrint/spawner/BP_spawner_4.BP_spawner_4_C" (Math|Transform|MakeTransform "-6670.000000,2750.000000,180.000000" "0, 0, 0" "0.100000,0.100000,0.100000") "Undefined" "MultiplyWithRoot" 0 0))))

(fn SpawnBlockSpawner1
  (Utilities|FlowControl|Sequence
    (:then_0
      (Game|SpawnActorfromClass "/Game/BluePrint/spawner/BP_spawner_Forword.BP_spawner_Forword_C" (Math|Transform|MakeTransform "2740.000000,-910.000000,-290.000000" "0, 0, 0" "0.100000,0.100000,0.100000") "Undefined" "MultiplyWithRoot" 0 0)
      (Game|SpawnActorfromClass "/Game/BluePrint/spawner/BP_spawner_Jump.BP_spawner_Jump_C" (Math|Transform|MakeTransform "2780.000000,-910.000000,-290.000000" "0, 0, 0" "0.100000,0.100000,0.100000") "Undefined" "MultiplyWithRoot" 0 0)
      (Game|SpawnActorfromClass "/Game/BluePrint/spawner/BP_spawner_LeftTurn.BP_spawner_LeftTurn_C" (Math|Transform|MakeTransform "2820.000000,-910.000000,-290.000000" "0, 0, 0" "0.100000,0.100000,0.100000") "Undefined" "MultiplyWithRoot" 0 0)
      (Game|SpawnActorfromClass "/Game/BluePrint/spawner/BP_spawner_RightTurn.BP_spawner_RightTurn_C" (Math|Transform|MakeTransform "2840.000000,-910.000000,-290.000000" "0, 0, 0" "0.100000,0.100000,0.100000") "Undefined" "MultiplyWithRoot" 0 0))
    (:then_1
      (Game|SpawnActorfromClass "/Game/BluePrint/spawner/BP_spawner_Loop.BP_spawner_Loop_C" (Math|Transform|MakeTransform "2740.000000,-910.000000,-250.000000" "0, 0, 0" "0.100000,0.100000,0.100000") "Undefined" "MultiplyWithRoot" 0 0)
      (Game|SpawnActorfromClass "/Game/BluePrint/spawner/BP_spawner_2.BP_spawner_2_C" (Math|Transform|MakeTransform "2780.000000,-910.000000,-250.000000" "0, 0, 0" "0.100000,0.100000,0.100000") "Undefined" "MultiplyWithRoot" 0 0)
      (Game|SpawnActorfromClass "/Game/BluePrint/spawner/BP_spawner_3.BP_spawner_3_C" (Math|Transform|MakeTransform "2820.000000,-910.000000,-250.000000" "0, 0, 0" "0.100000,0.100000,0.100000") "Undefined" "MultiplyWithRoot" 0 0)
      (Game|SpawnActorfromClass "/Game/BluePrint/spawner/BP_spawner_4.BP_spawner_4_C" (Math|Transform|MakeTransform "2840.000000,-910.000000,-250.000000" "0, 0, 0" "0.100000,0.100000,0.100000") "Undefined" "MultiplyWithRoot" 0 0))))