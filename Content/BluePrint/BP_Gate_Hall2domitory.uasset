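; BP_Gate_Hall2domitory is a level-transition gate, named for hall to dormitory, that opens the level set in LevelName when its box is overlapped.
; On BeginPlay it caches the BP_NPCManager actor.
; On overlap, if the SaveNpcData slot already exists, it copies the manager's NPC data into the save object and writes it before switching levels.
; The overlap is not filtered by actor, and no save is created when the slot is absent.
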(event OnComponentBeginOverlap(Box)
  (params (OverlappedComponent :type Primitive%20Component%20Object%20Reference) (OtherActor :type Actor%20Object%20Reference) (OtherComp :type Primitive%20Component%20Object%20Reference) (OtherBodyIndex :type Integer) (bFromSweep :type Boolean) (SweepResult :type Hit%20Result%20Structure%20%28by%20ref%29))
  (bind _npcdatamanager (Variables|Default|GetNPCDataManager))
  (bind _savenpcdata (Variables|/Game/BluePrint/NPC/BP_NPCManager.BP_NPCManager_C|GetSaveNpcData _npcdatamanager))
  (bind _returnvalue (SaveGame|DoesSaveGameExist "SaveNpcData"))
  (if _returnvalue
    (Variables|/Game/Quest/BP_SaveNPCData.BP_SaveNPCData_C|SetNPCData _savenpcdata (Variables|/Game/BluePrint/NPC/BP_NPCManager.BP_NPCManager_C|GetNPCData (Variables|Default|GetNPCDataManager)))
    (SaveGame|SaveGametoSlot _savenpcdata "SaveNpcData")
    (Development|PrintText "저장"))
  (Game|OpenLevel(byObjectReference) (Variables|Default|GetLevelName) false))

(event EventBeginPlay
  (bind _returnvalue (Actor|GetActorOfClass "/Game/BluePrint/NPC/BP_NPCManager.BP_NPCManager_C"))
  (Variables|Default|SetNPCDataManager _returnvalue))

(event Collision|EventActorBeginOverlap
  (params (OtherActor :type Actor%20Object%20Reference)))

(event EventTick
  (params (DeltaSeconds :type Float%20%28single-precision%29)))

(fn ConstructionScript)