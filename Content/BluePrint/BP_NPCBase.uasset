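; BP_NPCBase is an NPC Blueprint, named as a base, that carries dialog, dialog option and magic option widget components.
; On BeginPlay it casts each component's widget to its WBP class and caches the reference, stopping at the first failed cast.
; After a short delay it hides all three widgets; no logic here shows them again.
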(event EventBeginPlay
  (bind _aswbp_npcdialog (Utilities|Casting|CastToWBP_NPCDialog (UserInterface|GetUserWidgetObject (Variables|Default|GetDialogWidget))))
  (Variables|Default|SetAs%20WBP%20NPCDialog _aswbp_npcdialog)
  (bind _aswbp_dialog_option (Utilities|Casting|CastToWBP_DialogOption (UserInterface|GetUserWidgetObject (Variables|Default|GetDialogOptionWidget))))
  (Variables|Default|SetAs%20WBP%20Dialog%20Option _aswbp_dialog_option)
  (bind _aswbp_magic_option (Utilities|Casting|CastToWBP_MagicOption (UserInterface|GetUserWidgetObject (Variables|Default|GetMagicOptionWidget))))
  (Variables|Default|SetAs%20WBP%20Magic%20Option _aswbp_magic_option)
  (Utilities|FlowControl|Delay 0.5)
  (Widget|SetVisibility (Variables|Default|GetAs%20WBP%20NPCDialog) "Hidden")
  (Widget|SetVisibility (Variables|Default|GetAs%20WBP%20Dialog%20Option) "Hidden")
  (Widget|SetVisibility (Variables|Default|GetAs%20WBP%20Magic%20Option) "Hidden"))

(fn ConstructionScript)