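; Burning house actor that gets extinguished when the FireDie event fires or the T key is pressed.
; Water components start hidden, and Tick rebinds the Fin handler to FireDie every frame.
; Fin reveals the water and plays the EndFire timeline to drive the scale of three Niagara effects.
; A three-second delay chained to the timeline's Update then destroys the water components and the actor.
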(event Custom|Fin
  (Rendering|SetVisibility (Variables|Default|GetWater) true false)
  (Rendering|SetVisibility (Variables|Default|GetWater1) true false)
  (bind _새_트랙_0 (Timeline|EndFire PlayFromStart)
    (:Update
      (Transformation|SetWorldScale3D (Variables|Default|GetNiagara1) (Math|Vector|MakeVector _새_트랙_0 _새_트랙_0 _새_트랙_0))
      (Utilities|FlowControl|Delay 3.0)
      (Components|DestroyComponent (Variables|Default|GetWater))
      (Actor|DestroyActor))))

(event EventBeginPlay
  (Rendering|SetVisibility (Variables|Default|GetWater) false false)
  (Rendering|SetVisibility (Variables|Default|GetWater1) false false)
  (Input|EnableInput (Game|GetPlayerController 0)))

(event Collision|EventActorBeginOverlap
  (params (OtherActor :type Actor%20Object%20Reference)))

(event EventTick
  (params (DeltaSeconds :type Float%20%28single-precision%29))
  (EventDispatchers|BindEventtoFireDie (delegate Custom|Fin)))

(event Input|KeyboardEvents|T
  (params (Key :type Key%20Structure :default "None"))
  (:Pressed
    (Rendering|SetVisibility (Variables|Default|GetWater) true false)
    (Rendering|SetVisibility (Variables|Default|GetWater1) true false)
    (bind _새_트랙_0 (Timeline|EndFire PlayFromStart)
      (:Update
        (Transformation|SetWorldScale3D (Variables|Default|GetNiagara1) (Math|Vector|MakeVector _새_트랙_0 _새_트랙_0 _새_트랙_0))
        (Utilities|FlowControl|Delay 3.0)
        (Components|DestroyComponent (Variables|Default|GetWater))
        (Actor|DestroyActor)))))

(fn ConstructionScript)