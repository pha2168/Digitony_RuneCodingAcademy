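; BP_Rain is a rain effect actor that moves a Niagara component along a spline, then destroys itself.
; A Rain event or the M key restarts a timeline whose alpha sets the effect's world location and rotation along the spline's length.
; The timeline update also runs a six-second Delay into DestroyActor, and BeginPlay enables player input for the key trigger.
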(event Custom|Rain
  (bind _spline (Variables|Default|GetSpline))
  (bind _animationalpha (Timeline|타임라인 PlayFromStart)
    (:Update
      (Transformation|SetWorldTransform (Variables|Default|GetNiagara) (Math|Transform|MakeTransform (Spline|GetLocationatDistanceAlongSpline _spline (* (Spline|GetSplineLength _spline) _animationalpha) "World") (Spline|GetRotationatDistanceAlongSpline _spline (* (Spline|GetSplineLength _spline) _animationalpha) "World")) false false)
      (Utilities|FlowControl|Delay 6.0)
      (Actor|DestroyActor))))

(event EventBeginPlay
  (Input|EnableInput (Game|GetPlayerController 0)))

(event Collision|EventActorBeginOverlap
  (params (OtherActor :type Actor%20Object%20Reference)))

(event EventTick
  (params (DeltaSeconds :type Float%20%28single-precision%29)))

(event Input|KeyboardEvents|M
  (params (Key :type Key%20Structure :default "None"))
  (bind _spline (Variables|Default|GetSpline))
  (:Pressed
    (bind _animationalpha (Timeline|타임라인 PlayFromStart)
      (:Update
        (Transformation|SetWorldTransform (Variables|Default|GetNiagara) (Math|Transform|MakeTransform (Spline|GetLocationatDistanceAlongSpline _spline (* (Spline|GetSplineLength _spline) _animationalpha) "World") (Spline|GetRotationatDistanceAlongSpline _spline (* (Spline|GetSplineLength _spline) _animationalpha) "World")) false false)
        (Utilities|FlowControl|Delay 6.0)
        (Actor|DestroyActor)))))

(fn ConstructionScript)