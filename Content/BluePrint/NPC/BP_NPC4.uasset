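; BP_NPC4 is a quest NPC that shows dialogue to the VR player and spawns BP_Shaga once when its quest flag is set.
; It reads its entry from BP_NPCManager by DataIndex, with a delayed Tick syncing Plane visibility to the quest flag.
; Trigger overlap fills the dialogue, option and magic widgets and plays a one-time sound gated by quest state.
; Leaving the trigger hides the widgets.
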(event OnComponentEndOverlap(Triger)
  (params (OverlappedComponent :type Primitive%20Component%20Object%20Reference) (OtherActor :type Actor%20Object%20Reference) (OtherComp :type Primitive%20Component%20Object%20Reference) (OtherBodyIndex :type Integer))
  (Widget|SetVisibility (Variables|Default|GetAs%20WBP%20NPCDialog) "Hidden")
  (Widget|SetVisibility (Variables|Default|GetAs%20WBP%20Dialog%20Option) "Hidden")
  (Widget|SetVisibility (Variables|Default|GetAs%20WBP%20Magic%20Option) "Hidden")
  (Variables|Default|SetOverLap false))

(event OnComponentBeginOverlap(Triger)
  (params (OverlappedComponent :type Primitive%20Component%20Object%20Reference) (OtherActor :type Actor%20Object%20Reference) (OtherComp :type Primitive%20Component%20Object%20Reference) (OtherBodyIndex :type Integer) (bFromSweep :type Boolean) (SweepResult :type Hit%20Result%20Structure%20%28by%20ref%29))
  (bind _datamgr (Variables|Default|GetDataMgr))
  (bind _dataindex (Variables|Default|GetDataIndex))
  (bind _npcdata (Variables|/Game/BluePrint/NPC/BP_NPCManager.BP_NPCManager_C|GetNPCData _datamgr))
  (bind _output (Utilities|Array|Get(acopy) _npcdata _dataindex))
  (Utilities|Casting|CastToVRPawn OtherActor)
  (bind _output_get (Variables|Default|SetOverLap true))
  (Widget|SetVisibility (Variables|Default|GetAs%20WBP%20NPCDialog) "Visible")
  (Default|UpdateDialog (Variables|Default|GetAs%20WBP%20NPCDialog) (.nickname _output) (.name _output) (.dialog _output) (.firstdialog _output) (.bquest _output))
  (Default|QuestOptionVisiblity (Variables|Default|GetAs%20WBP%20Dialog%20Option) (and (.bquest _output) _output_get))
  (Default|SetMagicType (Variables|Default|GetAs%20WBP%20Magic%20Option) (.mgictype _output) _dataindex (.magicclicletransform _output) (.algorithmtransform _output) (.magicwidgettransform _output))
  (Default|GetIndex (Variables|Default|GetAs%20WBP%20Dialog%20Option) _dataindex)
  (Utilities|FlowControl|DoOnce (not (.bquest _output))
    (:Completed
      (Audio|PlaySound2D (Variables|Default|GetSound) 1.0 1.0 0.0 0 0))))

(event EventBeginPlay
  (|CallParentFunction)
  (Utilities|FlowControl|Delay 0.3)
  (bind _returnvalue (Actor|GetActorOfClass "/Game/BluePrint/NPC/BP_NPCManager.BP_NPCManager_C"))
  (Variables|Default|SetDataMgr _returnvalue)
  (if (and (.bquest (Utilities|Array|Get(acopy) (Variables|/Game/BluePrint/NPC/BP_NPCManager.BP_NPCManager_C|GetNPCData (Variables|Default|GetDataMgr)) (Variables|Default|GetDataIndex))) (Variables|Default|GetSpawn))
    (Game|SpawnActorfromClass "/Game/BluePrint/NPC/BP_Shaga.BP_Shaga_C" (Math|Transform|MakeTransform "1770.000000,-6940.000000,520.000000" "0, 0, 0" "1.000000,1.000000,1.000000") "Undefined" "MultiplyWithRoot" 0 0)
    (Variables|Default|SetSpawn false)))

(event EventTick
  (params (DeltaSeconds :type Float%20%28single-precision%29))
  (bind _datamgr (Variables|Default|GetDataMgr))
  (bind _dataindex (Variables|Default|GetDataIndex))
  (bind _npcdata (Variables|/Game/BluePrint/NPC/BP_NPCManager.BP_NPCManager_C|GetNPCData _datamgr))
  (bind _output (Utilities|Array|Get(acopy) _npcdata _dataindex))
  (Utilities|FlowControl|Delay 0.2)
  (Rendering|SetVisibility (Variables|Default|GetPlane) (.bquest _output) false)
  (if (and (.bquest _output) (Variables|Default|GetSpawn))
    (Game|SpawnActorfromClass "/Game/BluePrint/NPC/BP_Shaga.BP_Shaga_C" (Math|Transform|MakeTransform "1770.000000,-6940.000000,520.000000" "0, 0, 0" "1.000000,1.000000,1.000000") "Undefined" "MultiplyWithRoot" 0 0)
    (Variables|Default|SetSpawn false)))

(fn ConstructionScript
  (|CallParentFunction))