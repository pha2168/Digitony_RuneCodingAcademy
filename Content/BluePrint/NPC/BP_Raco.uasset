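; BP_Raco is an NPC actor whose skeletal mesh is hidden at BeginPlay and flown or moved along a spline by a Move event.
; Move spawns a BP_Wind at a fixed world transform and plays a timeline whose alpha drives the mesh's position and rotation by spline distance.
; A Delay on the timeline's update destroys the wind after a few seconds.
; Nothing in this Blueprint makes the mesh visible again.
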(event Custom|Move
  (bind _spline (Variables|Default|GetSpline))
  (bind _returnvalue (Game|SpawnActorfromClass "/Game/BluePrint/NPC/BP_Wind.BP_Wind_C" (Math|Transform|MakeTransform "5280.000000,9710.000000,2330.000000" "-12.000000,35.000000,-142.000000" "0.300000,0.300000,0.300000") "Undefined" "MultiplyWithRoot" 0 0))
  (bind _animationalpha (Timeline|타임라인 Play)
    (:Update
      (Transformation|SetWorldTransform (Variables|Default|GetSkeletalMesh) (Math|Transform|MakeTransform (Spline|GetLocationatDistanceAlongSpline _spline (* (Spline|GetSplineLength _spline) _animationalpha) "World") (Spline|GetRotationatDistanceAlongSpline _spline (* (Spline|GetSplineLength _spline) _animationalpha) "World") "2.500000,2.500000,2.500000") false false)
      (Utilities|FlowControl|Delay 3.0)
      (Actor|DestroyActor _returnvalue))))

(event EventBeginPlay
  (Rendering|SetVisibility (Variables|Default|GetSkeletalMesh) false false))

(event Collision|EventActorBeginOverlap
  (params (OtherActor :type Actor%20Object%20Reference)))

(event EventTick
  (params (DeltaSeconds :type Float%20%28single-precision%29)))

(fn ConstructionScript)