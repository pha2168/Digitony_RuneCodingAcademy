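; BP_Shaga is an NPC actor that flies or travels its skeletal mesh along its spline, accompanied by a spawned BP_Wind effect actor.
; The move event, or the N key via input enabled on BeginPlay, spawns the wind at the actor's transform and starts a timeline.
; Each timeline update sets the mesh's position and rotation along the spline.
; A Delay on that update path destroys both actors three seconds after movement begins.
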(event Custom|move
  (bind _returnvalue (Transformation|GetActorTransform))
  (bind _spline (Variables|Default|GetSpline))
  (bind _returnvalue_2 (Game|SpawnActorfromClass "/Game/BluePrint/NPC/BP_Wind.BP_Wind_C" (Math|Transform|MakeTransform (.location _returnvalue) (.rotation _returnvalue) "2.000000,2.000000,2.000000") "Undefined" "MultiplyWithRoot" 0 0))
  (bind _새_트랙_0 (Timeline|타임라인 PlayFromStart)
    (:Update
      (Transformation|SetWorldTransform (Variables|Default|GetSkeletalMesh) (Math|Transform|MakeTransform (Spline|GetLocationatDistanceAlongSpline _spline (* (Spline|GetSplineLength _spline) _새_트랙_0) "World") (Spline|GetRotationatDistanceAlongSpline _spline (* (Spline|GetSplineLength _spline) _새_트랙_0) "World") "15.000000,15.000000,15.000000") false false)
      (Utilities|FlowControl|Delay 3.0)
      (Actor|DestroyActor _returnvalue_2)
      (Actor|DestroyActor))))

(event EventBeginPlay
  (Input|EnableInput (Game|GetPlayerController 0)))

(event EventTick
  (params (DeltaSeconds :type Float%20%28single-precision%29)))

(event Input|KeyboardEvents|N
  (params (Key :type Key%20Structure :default "None"))
  (bind _returnvalue (Transformation|GetActorTransform))
  (bind _spline (Variables|Default|GetSpline))
  (:Pressed
    (bind _returnvalue_2 (Game|SpawnActorfromClass "/Game/BluePrint/NPC/BP_Wind.BP_Wind_C" (Math|Transform|MakeTransform (.location _returnvalue) (.rotation _returnvalue) "2.000000,2.000000,2.000000") "Undefined" "MultiplyWithRoot" 0 0))
    (bind _새_트랙_0 (Timeline|타임라인 PlayFromStart)
      (:Update
        (Transformation|SetWorldTransform (Variables|Default|GetSkeletalMesh) (Math|Transform|MakeTransform (Spline|GetLocationatDistanceAlongSpline _spline (* (Spline|GetSplineLength _spline) _새_트랙_0) "World") (Spline|GetRotationatDistanceAlongSpline _spline (* (Spline|GetSplineLength _spline) _새_트랙_0) "World") "15.000000,15.000000,15.000000") false false)
        (Utilities|FlowControl|Delay 3.0)
        (Actor|DestroyActor _returnvalue_2)
        (Actor|DestroyActor)))))

(fn ConstructionScript)