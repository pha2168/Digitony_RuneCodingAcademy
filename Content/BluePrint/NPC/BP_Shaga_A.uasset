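; BP_Shaga_A is an NPC actor that moves its skeletal mesh along a spline when its Die event fires, then destroys itself.
; Tick rebinds the Animetion event to Die every frame instead of binding once.
; Animetion plays a timeline whose track drives spline distance for world location and rotation.
; A Delay on the timeline's Update pin destroys the actor seconds after playback starts, independent of timeline completion.
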(event Custom|Animetion
  (bind _spline (Variables|Default|GetSpline))
  (bind _새_트랙_0 (Timeline|타임라인 Play)
    (:Update
      (Transformation|SetWorldTransform (Variables|SkeletalMeshActor|GetSkeletalMeshComponent) (Math|Transform|MakeTransform (Spline|GetLocationatDistanceAlongSpline _spline (* (Spline|GetSplineLength _spline) _새_트랙_0) "World") (Spline|GetRotationatDistanceAlongSpline _spline (* (Spline|GetSplineLength _spline) _새_트랙_0) "World")) false false)
      (Utilities|FlowControl|Delay 3.0)
      (Actor|DestroyActor))))

(event EventBeginPlay)

(event Collision|EventActorBeginOverlap
  (params (OtherActor :type Actor%20Object%20Reference)))

(event EventTick
  (params (DeltaSeconds :type Float%20%28single-precision%29))
  (EventDispatchers|BindEventtoDie (delegate Custom|Animetion)))

(fn ConstructionScript)