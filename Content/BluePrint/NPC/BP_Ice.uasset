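; BP_Ice is an ice actor that reacts to the ClearMapIce event with a fire effect and a scale-down animation.
; It rebinds its Get event to ClearMapIce every Tick.
; Get shows fire Niagara effects on VRPawn and BP_Character while the GettingSmall timeline rescales two particle systems.
; A three-second Delay on the timeline's Update then hides those Niagara effects.
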(event Custom|get
  (Utilities|FlowControl|Sequence
    (:then_0
      (bind _returnvalue (Actor|GetActorOfClass "/Game/VRTemplate/Blueprints/VRPawn.VRPawn_C")))
    (:then_1
      (bind _returnvalue_2 (Actor|GetActorOfClass "/Game/BluePrint/test/BP_Character.BP_Character_C"))))
  (Rendering|SetVisibility (Variables|/Game/VRTemplate/Blueprints/VRPawn.VRPawn_C|GetFire_Niagara _returnvalue) true false)
  (bind _새_트랙_0 (Timeline|gettingSmall Play)
    (:Update
      (Transformation|SetWorldScale3D (Variables|Default|GetParticleSystem1) (Math|Vector|MakeVector _새_트랙_0 _새_트랙_0 _새_트랙_0))
      (Utilities|FlowControl|Delay 3.0)
      (Rendering|SetVisibility (Variables|/Game/VRTemplate/Blueprints/VRPawn.VRPawn_C|GetFire_Niagara _returnvalue) false false))))

(event EventBeginPlay)

(event EventTick
  (params (DeltaSeconds :type Float%20%28single-precision%29))
  (EventDispatchers|BindEventtoClearMapIce (delegate Custom|get)))

(fn ConstructionScript)