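; BP_SplineActorBase is a base actor that moves a static mesh along its spline.
; The play event runs a timeline from the start, whose AnimationAlpha scales the spline length into a distance that sets the mesh's world location and rotation at unit scale.
; Play is bound to the PlaySpline event on Tick, so the binding call repeats every frame.
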(event Custom|play
  (bind _spline (Variables|Default|GetSpline))
  (bind _animationalpha (Timeline|타임라인 PlayFromStart)
    (:Update
      (Transformation|SetWorldTransform (Variables|Default|GetStaticMesh) (Math|Transform|MakeTransform (Spline|GetLocationatDistanceAlongSpline _spline (* (Spline|GetSplineLength _spline) _animationalpha) "World") (Spline|GetRotationatDistanceAlongSpline _spline (* (Spline|GetSplineLength _spline) _animationalpha) "World")) false false))))

(event EventTick
  (params (DeltaSeconds :type Float%20%28single-precision%29))
  (EventDispatchers|BindEventtoPlaySpline (delegate Custom|play)))

(fn ConstructionScript)