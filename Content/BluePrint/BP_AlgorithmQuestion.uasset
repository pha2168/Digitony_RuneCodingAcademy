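; BP_AlgorithmQuestion is a code-block magic puzzle map with five selectable data sets, built in the construction script via LoadMapData and CreateMap.
; GetIndexData picks the map data, reloads it and stores the puzzle index.
; FinishMagic removes code blocks, spawners and the magic widget, has the magic circle evaluate the score and teleports it away, then clears the map.
; The index then selects the world payoff: spline playback, ice clearing, fire extinguishing, Shaga death or dormitory darkness removal.
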(event EventBeginPlay
  (bind _returnvalue (Actor|GetActorOfClass "/Game/BluePrint/BP_MagicCircle.BP_MagicCircle_C"))
  (Variables|Default|SetMagicCircle _returnvalue)
  (bind _returnvalue_2 (Actor|GetActorOfClass "/Game/BluePrint/test/BP_MagicLuni.BP_MagicLuni_C"))
  (Variables|Default|SetLuni _returnvalue_2))

(event Collision|EventActorBeginOverlap
  (params (OtherActor :type Actor%20Object%20Reference)))

(event EventTick
  (params (DeltaSeconds :type Float%20%28single-precision%29)))

(event EventFinishMagic
  (bind _outactors (Actor|GetAllActorsOfClass "/Game/BluePrint/CodeBlock/BP_CodeBlockBase.BP_CodeBlockBase_C"))
  (for _array_element _outactors
    (Actor|DestroyActor _array_element))
  (bind _outactors_2 (Actor|GetAllActorsOfClass "/Game/BluePrint/spawner/BP_spawner.BP_spawner_C"))
  (for _array_element_2 _outactors_2
    (Actor|DestroyActor _array_element_2))
  (bind _returnvalue (Actor|GetActorOfClass "/Game/BluePrint/BP_MagicWiget.BP_MagicWiget_C"))
  (Actor|DestroyActor _returnvalue)
  (bind _returnvalue_2 (Actor|GetActorOfClass "/Game/BluePrint/BP_MagicCircle.BP_MagicCircle_C"))
  (Class|CMagicCircle|EvaluateScore _returnvalue_2)
  (Transformation|Teleport _returnvalue_2 "0.000000,-1000.000000,0.000000" "0, 0, 0")
  (Class|CAlgorithmQuestion|ClearMap)
  (Development|PrintText "맵 클리어")
  (switch int (Variables|Default|GetIndex)
    (:0
      (bind _outactors_3 (Actor|GetAllActorsOfClass "/Game/BluePrint/SplineActor/BP_SplineActorBase.BP_SplineActorBase_C"))
      (for _array_element_3 _outactors_3
        (Default|CallPlaySpline _array_element_3)))
    (:1
      (bind _outactors_4 (Actor|GetAllActorsOfClass "/Game/BluePrint/NPC/BP_Ice.BP_Ice_C"))
      (for _array_element_4 _outactors_4
        (Default|CallClearMapIce _array_element_4)))
    (:2
      (bind _outactors_5 (Actor|GetAllActorsOfClass "/Game/BluePrint/NPC/BP_FireHoues.BP_FireHoues_C"))
      (for _array_element_5 _outactors_5
        (Default|CallFireDie _array_element_5)))
    (:3
      (bind _outactors_6 (Actor|GetAllActorsOfClass "/Game/BluePrint/NPC/BP_Shaga_A.BP_Shaga_A_C"))
      (for _array_element_6 _outactors_6
        (Default|CallDie _array_element_6)))
    (:4
      (bind _outactors_7 (Actor|GetAllActorsOfClass "/Game/BluePrint/NPC/BP_DomitoryDark.BP_DomitoryDark_C"))
      (for _array_element_7 _outactors_7
        (Actor|DestroyActor _array_element_7)))))

(fn ConstructionScript
  (Class|CAlgorithmQuestion|LoadMapData)
  (Class|CAlgorithmQuestion|CreateMap))

(fn GetIndexData
  (params (DataIndex :type Integer))
  (switch int DataIndex
    (:0
      (Variables|Default|SetMapData (Variables|Default|GetMapData1)))
    (:1
      (Variables|Default|SetMapData (Variables|Default|GetMapData2)))
    (:2
      (Variables|Default|SetMapData (Variables|Default|GetMapData3)))
    (:3
      (Variables|Default|SetMapData (Variables|Default|GetMapData4)))
    (:4
      (Variables|Default|SetMapData (Variables|Default|GetMapData5))))
  (Class|CAlgorithmQuestion|LoadMapData)
  (Variables|Default|SetIndex DataIndex))