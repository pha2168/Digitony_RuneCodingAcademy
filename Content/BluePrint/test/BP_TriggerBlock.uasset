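; BP_TriggerBlock is a one-shot player trigger with a static mesh that starts hidden and a box overlap volume.
; When the player character enters the box, the mesh shows briefly, then hides as a 2D sound plays.
; It then finds BP_AIController by class, sets its PlayerGoalCheck blackboard key to false, and destroys itself.
; A CallTrigger call is left unconnected and never runs.
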(event OnComponentBeginOverlap(Box)
  (params (OverlappedComponent :type Primitive%20Component%20Object%20Reference) (OtherActor :type Actor%20Object%20Reference) (OtherComp :type Primitive%20Component%20Object%20Reference) (OtherBodyIndex :type Integer) (bFromSweep :type Boolean) (SweepResult :type Hit%20Result%20Structure%20%28by%20ref%29))
  (if (== OtherActor (Game|GetPlayerCharacter 0))
    (Rendering|SetVisibility (Variables|Default|GetStaticMesh) true false)
    (Utilities|FlowControl|Delay 1.0)
    (Rendering|SetVisibility (Variables|Default|GetStaticMesh) false false)
    (Audio|PlaySound2D "/Game/Sound/Luni_sound/루니__마법숲으로가자_.루니__마법숲으로가자_" 1.0 1.0 0.0 0 0)
    (bind _returnvalue (Actor|GetActorOfClass "/Game/BluePrint/BP_AIController.BP_AIController_C"))
    (AI|Components|Blackboard|SetValueasBool (AI|GetBlackboard (AI|GetAIController _returnvalue)) (Variables|Default|GetPlayerGoalCheck) false)
    (Actor|DestroyActor)))

(event EventBeginPlay
  (Rendering|SetVisibility (Variables|Default|GetStaticMesh) false false))

(event Collision|EventActorBeginOverlap
  (params (OtherActor :type Actor%20Object%20Reference)))

(event EventTick
  (params (DeltaSeconds :type Float%20%28single-precision%29)))

(fn ConstructionScript)