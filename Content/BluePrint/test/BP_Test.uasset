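; BP_Test is a debug actor that enables player input on BeginPlay to trigger scene effects manually.
; Pressing T calls Move on every BP_Shaga and plays a wind magic sound for each.
; Several unconnected chains hold similar triggers for spline, fire, ice, darkness and Raco actors, most with elemental magic sounds.
; Two other unconnected chains spawn actors at fixed locations, one being a BP_Rain that starts raining.
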(event EventBeginPlay
  (Input|EnableInput (Game|GetPlayerController 0)))

(event EventTick
  (params (DeltaSeconds :type Float%20%28single-precision%29)))

(event Input|KeyboardEvents|T
  (params (Key :type Key%20Structure :default "None"))
  (:Pressed
    (bind _outactors (Actor|GetAllActorsOfClass "/Game/BluePrint/NPC/BP_Shaga.BP_Shaga_C"))
    (for _array_element _outactors
      (Default|Move _array_element)
      (Audio|PlaySound2D "/Game/Sound/게임_효과음_WAV/MP_바람-속성-마법.MP_바람-속성-마법" 1.0 1.0 0.0 0 0))))

(fn ConstructionScript)