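; Magic circle actor for a block-coding puzzle that displays queued code blocks as icons and triggers their execution.
; UpdateMagicCircle adds a mesh component, then maps each Forward, Turn or Jump block to an icon at one of 16 transforms cached at BeginPlay.
; Z calls StartMagic on BP_AlgorithmQuestion.
; Move, rebound every Tick, teleports the circle, switches to water Niagara and spawns the question actor after a delay.
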(event Custom|Move
  (Transformation|Teleport "80.000000,0.000000,100.000000" "0, 0, 0")
  (Class|NiagaraComponent|SetAsset (Variables|Default|GetNiagara) "/Game/VFX/Niagara/NS_Magic_water.NS_Magic_water" true)
  (Utilities|FlowControl|Delay 2.0)
  (Game|SpawnActorfromClass "/Game/BluePrint/BP_AlgorithmQuestion.BP_AlgorithmQuestion_C" (Math|Transform|MakeTransform "60.000000,-30.000000,80.000000" "0, 0, 0" "1.000000,1.000000,1.000000") "Undefined" "MultiplyWithRoot" 0 0))

(event EventBeginPlay
  (Input|EnableInput (Game|GetPlayerController 0))
  (CallFunction|GetTransBlock)
  (Utilities|Array|Clear (Variables|Default|GetCodeBlocks)))

(event EventUpdateMagicCircle
  (bind _codeblockarray (Variables|Default|GetCodeBlockArray))
  (bind _returnvalue (AddComponent|AddStaticMeshComponent false))
  (Utilities|Array|Add _codeblockarray _returnvalue)
  (for _array_element _codeblockarray
    (Components|StaticMesh|SetStaticMesh _array_element 0)
    (for (_array_element_2 _array_index) (Variables|Default|GetCodeBlocks)
      (switch Utilities|FlowControl|Switch|SwitchonECodeBlockType (.CodeBlockType (Utilities|Struct|BreakCodeBlockInfo _array_element_2))
        (:Forward
          (Components|StaticMesh|SetStaticMesh (Utilities|Array|Get(acopy) (Variables|Default|GetCodeBlockArray) _array_index) "/Game/Meshes/newblock/esset/GOblock_Point.GOblock_Point")
          (Transformation|SetWorldTransform (Utilities|Array|Get(acopy) (Variables|Default|GetCodeBlockArray) _array_index) (Math|Transform|MakeTransform (.location (Utilities|Array|Get(acopy) (Variables|Default|GetCodeBlockIconTransform) _array_index)) "0.000000,90.000000,90.000000" "0.100000,0.100000,0.100000") false false))
        (:RightTurn
          (Components|StaticMesh|SetStaticMesh (Utilities|Array|Get(acopy) (Variables|Default|GetCodeBlockArray) _array_index) "/Game/Meshes/newblock/esset/TurnRightblock_Point.TurnRightblock_Point")
          (Transformation|SetWorldTransform (Utilities|Array|Get(acopy) (Variables|Default|GetCodeBlockArray) _array_index) (Math|Transform|MakeTransform (.location (Utilities|Array|Get(acopy) (Variables|Default|GetCodeBlockIconTransform) _array_index)) "0.000000,90.000000,90.000000" "0.080000,0.080000,0.080000") false false :!label _label))
        (:LeftTurn
          (Components|StaticMesh|SetStaticMesh (Utilities|Array|Get(acopy) (Variables|Default|GetCodeBlockArray) _array_index) "/Game/Meshes/newblock/esset/TurnLeftblock_Point.TurnLeftblock_Point")
          (goto _label))
        (:Jump
          (Components|StaticMesh|SetStaticMesh (Utilities|Array|Get(acopy) (Variables|Default|GetCodeBlockArray) _array_index) "/Game/Meshes/newblock/esset/jump.jump")
          (Transformation|SetWorldTransform (Utilities|Array|Get(acopy) (Variables|Default|GetCodeBlockArray) _array_index) (Math|Transform|MakeTransform (.location (Utilities|Array|Get(acopy) (Variables|Default|GetCodeBlockIconTransform) _array_index)) "0.000000,90.000000,0.000000" "0.180000,0.180000,0.180000") false false))))))

(event EventTick
  (params (DeltaSeconds :type Float%20%28single-precision%29))
  (EventDispatchers|BindEventtoMoveClicle (delegate Custom|Move)))

(event Input|KeyboardEvents|Z
  (params (Key :type Key%20Structure :default "None"))
  (:Pressed
    (bind _returnvalue (Actor|GetActorOfClass "/Game/BluePrint/BP_AlgorithmQuestion.BP_AlgorithmQuestion_C"))
    (Class|CAlgorithmQuestion|StartMagic _returnvalue)
    (Development|PrintText "마법 실행")))

(fn ConstructionScript)

(fn GetTransBlock
  (Utilities|Array|Add (Variables|Default|GetCodeBlockIconTransform) (Transformation|GetWorldTransform (Variables|Default|GetCodeBlock_01)))
  (Utilities|Array|Add (Variables|Default|GetCodeBlockIconTransform) (Transformation|GetWorldTransform (Variables|Default|GetCodeBlock_02)))
  (Utilities|Array|Add (Variables|Default|GetCodeBlockIconTransform) (Transformation|GetWorldTransform (Variables|Default|GetCodeBlock_03)))
  (Utilities|Array|Add (Variables|Default|GetCodeBlockIconTransform) (Transformation|GetWorldTransform (Variables|Default|GetCodeBlock_04)))
  (Utilities|Array|Add (Variables|Default|GetCodeBlockIconTransform) (Transformation|GetWorldTransform (Variables|Default|GetCodeBlock_05)))
  (Utilities|Array|Add (Variables|Default|GetCodeBlockIconTransform) (Transformation|GetWorldTransform (Variables|Default|GetCodeBlock_06)))
  (Utilities|Array|Add (Variables|Default|GetCodeBlockIconTransform) (Transformation|GetWorldTransform (Variables|Default|GetCodeBlock_07)))
  (Utilities|Array|Add (Variables|Default|GetCodeBlockIconTransform) (Transformation|GetWorldTransform (Variables|Default|GetCodeBlock_08)))
  (Utilities|Array|Add (Variables|Default|GetCodeBlockIconTransform) (Transformation|GetWorldTransform (Variables|Default|GetCodeBlock_09)))
  (Utilities|Array|Add (Variables|Default|GetCodeBlockIconTransform) (Transformation|GetWorldTransform (Variables|Default|GetCodeBlock_010)))
  (Utilities|Array|Add (Variables|Default|GetCodeBlockIconTransform) (Transformation|GetWorldTransform (Variables|Default|GetCodeBlock_011)))
  (Utilities|Array|Add (Variables|Default|GetCodeBlockIconTransform) (Transformation|GetWorldTransform (Variables|Default|GetCodeBlock_012)))
  (Utilities|Array|Add (Variables|Default|GetCodeBlockIconTransform) (Transformation|GetWorldTransform (Variables|Default|GetCodeBlock_013)))
  (Utilities|Array|Add (Variables|Default|GetCodeBlockIconTransform) (Transformation|GetWorldTransform (Variables|Default|GetCodeBlock_014)))
  (Utilities|Array|Add (Variables|Default|GetCodeBlockIconTransform) (Transformation|GetWorldTransform (Variables|Default|GetCodeBlock_015)))
  (Utilities|Array|Add (Variables|Default|GetCodeBlockIconTransform) (Transformation|GetWorldTransform (Variables|Default|GetCodeBlock_016))))