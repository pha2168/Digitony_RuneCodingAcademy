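; BP_NPC_Final is a quest NPC that shows dialog when a VR pawn enters its trigger.
; It fills the dialog widget from a fixed entry in BP_NPCManager's NPC data.
; If that entry's quest flag is set, it also reveals a final widget and plays a 2D sound once.
; Both widgets start hidden and are hidden again when a trigger overlap ends.
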(event OnComponentBeginOverlap(Trigger)
  (params (OverlappedComponent :type Primitive%20Component%20Object%20Reference) (OtherActor :type Actor%20Object%20Reference) (OtherComp :type Primitive%20Component%20Object%20Reference) (OtherBodyIndex :type Integer) (bFromSweep :type Boolean) (SweepResult :type Hit%20Result%20Structure%20%28by%20ref%29))
  (bind _datamgr (Variables|Default|GetDataMgr))
  (bind _npcdata (Variables|/Game/BluePrint/NPC/BP_NPCManager.BP_NPCManager_C|GetNPCData _datamgr))
  (bind _output (Utilities|Array|Get(acopy) _npcdata 8))
  (Utilities|Casting|CastToVRPawn OtherActor)
  (Rendering|SetVisibility (Variables|Default|GetDialog) true false)
  (Default|UpdateDialog (Variables|Default|GetAs%20WBP%20NPCDialog) (.nickname _output) (.name _output) (.dialog _output) (.firstdialog _output) (.bquest _output))
  (if (.bquest _output)
    (Rendering|SetVisibility (Variables|Default|GetFinalWidget) true false)
    (Utilities|FlowControl|DoOnce (not false)
      (:Completed
        (Audio|PlaySound2D 0 1.0 1.0 0.0 0 0)))))

(event OnComponentEndOverlap(Trigger)
  (params (OverlappedComponent :type Primitive%20Component%20Object%20Reference) (OtherActor :type Actor%20Object%20Reference) (OtherComp :type Primitive%20Component%20Object%20Reference) (OtherBodyIndex :type Integer))
  (Rendering|SetVisibility (Variables|Default|GetDialog) false false)
  (Rendering|SetVisibility (Variables|Default|GetFinalWidget) false false))

(event EventBeginPlay
  (Rendering|SetVisibility (Variables|Default|GetDialog) false false)
  (bind _aswbp_npcdialog (Utilities|Casting|CastToWBP_NPCDialog (UserInterface|GetUserWidgetObject (Variables|Default|GetDialog))))
  (Variables|Default|SetAs%20WBP%20NPCDialog _aswbp_npcdialog)
  (bind _returnvalue (Actor|GetActorOfClass "/Game/BluePrint/NPC/BP_NPCManager.BP_NPCManager_C"))
  (Variables|Default|SetDataMgr _returnvalue)
  (Utilities|FlowControl|Delay 0.2)
  (Rendering|SetVisibility (Variables|Default|GetFinalWidget) false false))

(fn ConstructionScript)