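; BP_NPC_6_1 is a quest NPC that shows its dialog when the VR player comes near.
; BeginPlay hides the Dialog component and caches the level's BP_NPCManager as DataMgr, which the graph does not otherwise use.
; The Trigger component reveals Dialog when a VRPawn begins overlapping and hides it when any overlap ends, without checking which actor left.
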(event OnComponentBeginOverlap(Trigger)
  (params (OverlappedComponent :type Primitive%20Component%20Object%20Reference) (OtherActor :type Actor%20Object%20Reference) (OtherComp :type Primitive%20Component%20Object%20Reference) (OtherBodyIndex :type Integer) (bFromSweep :type Boolean) (SweepResult :type Hit%20Result%20Structure%20%28by%20ref%29))
  (Utilities|Casting|CastToVRPawn OtherActor)
  (Rendering|SetVisibility (Variables|Default|GetDialog) true false))

(event OnComponentEndOverlap(Trigger)
  (params (OverlappedComponent :type Primitive%20Component%20Object%20Reference) (OtherActor :type Actor%20Object%20Reference) (OtherComp :type Primitive%20Component%20Object%20Reference) (OtherBodyIndex :type Integer))
  (Rendering|SetVisibility (Variables|Default|GetDialog) false false))

(event EventBeginPlay
  (Rendering|SetVisibility (Variables|Default|GetDialog) false false)
  (bind _returnvalue (Actor|GetActorOfClass "/Game/BluePrint/NPC/BP_NPCManager.BP_NPCManager_C"))
  (Variables|Default|SetDataMgr _returnvalue))

(fn ConstructionScript)